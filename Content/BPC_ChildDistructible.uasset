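; Child Blueprint actor of a destructible parent that changes its cube's material each time it is hit.
; The Hit event runs the parent logic, then applies the next entry in the Materials array to Cube and increments ArrayIndex.
; Material changes stop once the index reaches the end of the array, and each new index is printed for debugging.
; Tick and the construction script only call the parent.
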(event EventBeginPlay
  (|CallParentFunction) ; This node is disabled and will not be called.\nDrag off pins to build functionality.
)

(event Collision|EventActorBeginOverlap
  (params (OtherActor :type Actor%20Object%20Reference))
  (|CallParentFunction OtherActor) ; This node is disabled and will not be called.\nDrag off pins to build functionality.
)

(event EventTick
  (params (DeltaSeconds :type Float%20%28single-precision%29))
  (|CallParentFunction DeltaSeconds))

(event Collision|EventHit
  (params (MyComp :type Primitive%20Component%20Object%20Reference) (Other :type Actor%20Object%20Reference) (OtherComp :type Primitive%20Component%20Object%20Reference) (bSelfMoved :type Boolean) (HitLocation :type Vector :default "0, 0, 0") (HitNormal :type Vector :default "0, 0, 0") (NormalImpulse :type Vector :default "0, 0, 0") (Hit :type Hit%20Result%20Structure%20%28by%20ref%29))
  (|CallParentFunction MyComp Other OtherComp bSelfMoved HitLocation HitNormal NormalImpulse Hit)
  (if (< (Variables|Default|GetArrayIndex) (Utilities|Array|Length (Variables|Default|GetMaterials)))
    (bind _cube (Variables|Default|GetCube)
      (:then
        (Rendering|Material|SetMaterial _cube 0 (Utilities|Array|Get(acopy) (Variables|Default|GetMaterials) (Variables|Default|GetArrayIndex)))
        (bind _result (Math|Integer|IncrementInt (Variables|Default|GetArrayIndex))
          (:%20%20
            (bind _output_get (Variables|Default|SetArrayIndex _result))
            (Development|PrintString (Utilities|String|ToString(Integer) _output_get) true true "(R=0.000000,G=0.660000,B=1.000000,A=1.000000)" 5.0))))
      (:else))))

(fn ConstructionScript
  (|CallParentFunction))