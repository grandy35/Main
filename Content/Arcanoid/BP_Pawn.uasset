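; Player paddle pawn for an Arkanoid-style game that moves sideways and spawns the ball.
; The left and right axis inputs shift it along world X by a fixed, unswept step, not scaled by axis magnitude or frame time.
; On BeginPlay, SpawnBall creates a BP_Ball at the capsule's transform, stores it as PlayingBall and binds to its OnDead event.
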(event EventBeginPlay
  (CallFunction|SpawnBall))

(event Collision|EventActorBeginOverlap
  (params (OtherActor :type Actor%20Object%20Reference)))

(event EventTick
  (params (DeltaSeconds :type Float%20%28single-precision%29)))

(event Input|AxisEvents|InputAxisleft
  (params (AxisValue :type Float%20%28single-precision%29))
  (if (< AxisValue 0.0)
    (Transformation|AddActorWorldOffset "-50.000000,0.000000, 0")))

(event Input|AxisEvents|InputAxisright
  (params (AxisValue :type Float%20%28single-precision%29))
  (if (> AxisValue 0.0)
    (Transformation|AddActorWorldOffset "50.000000,0.000000, 0")))

(fn ConstructionScript)

(fn SpawnBall
  (bind _returnvalue (Game|SpawnActorfromClass "/Game/BP_Ball.BP_Ball_C" (Transformation|GetWorldTransform (Variables|Default|GetCapsule)) "AlwaysSpawn" 0 0))
  (bind _output_get (Variables|Default|SetPlayingBall _returnvalue))
  (EventDispatchers|BindEventtoOnDead _output_get (EventDispatchers|CreateEvent :!event SpawnBall))
  (return))