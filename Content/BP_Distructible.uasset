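; BP_Distructible is a breakable object that loses health when hit and removes its Cube component once worn down.
; Each Hit event applies BaseDamage to the actor itself and subtracts the value ApplyDamage returns from Health.
; While Health stays above ThresholdHP it prints the remaining value; otherwise it destroys the Cube component rather than the whole actor.
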(event EventBeginPlay)

(event EventTick
  (params (DeltaSeconds :type Float%20%28single-precision%29)))

(event Collision|EventHit
  (params (MyComp :type Primitive%20Component%20Object%20Reference) (Other :type Actor%20Object%20Reference) (OtherComp :type Primitive%20Component%20Object%20Reference) (bSelfMoved :type Boolean) (HitLocation :type Vector :default "0, 0, 0") (HitNormal :type Vector :default "0, 0, 0") (NormalImpulse :type Vector :default "0, 0, 0") (Hit :type Hit%20Result%20Structure%20%28by%20ref%29))
  (bind _self self)
  (bind _returnvalue (Game|Damage|ApplyDamage _self (Variables|Default|GetBaseDamage) 0 _self))
  (bind _output_get (Variables|Default|SetHealth (- (Variables|Default|GetHealth) _returnvalue)))
  (if (> _output_get (Variables|Default|GetThresholdHP))
    (Development|PrintString (Utilities|String|ToString(Float) (Variables|Default|GetHealth)))
    (else
      (Components|DestroyComponent (Variables|Default|GetCube)))))

(fn ConstructionScript)